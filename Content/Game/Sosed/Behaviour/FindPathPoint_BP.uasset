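; Behavior tree task that finds the current patrol point for a Yhizi_CBP_2 AI pawn.
; It reads the path index from the blackboard, transforms that PatrolPath point from the path actor's local space to world space, and writes it to a blackboard vector key.
; It finishes with success only when the path is valid; a failed cast or missing path never calls FinishExecute.
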(event `self.ReceiveExecuteAI`
  (params (OwnerController :type "AIController Object Reference") (ControlledPawn :type "Pawn Object Reference"))
  (bind _asyhizi_cbp_2 (cast `/Game/Game/Blueprints/Yhizi/Yhizi_CBP_2` ControlledPawn))
  (bind _patrolpath (`/Game/Game/Blueprints/Yhizi/Yhizi_CBP_2.PatrolPath` _asyhizi_cbp_2)
    (:`then`
      (`BTFunctionLibrary.SetBlackboardValueAsVector` (`self.BB_PathVector`) (`KismetMathLibrary.TransformLocation` (`Actor.GetTransform` _patrolpath) (`|GetArrayItem` (`/Game/Game/Sosed/Behaviour/PatrolPath.PathPoints` _patrolpath) (`BTFunctionLibrary.GetBlackboardValueAsInt` (`self.BB_PathIndex`)))))
      (`self.FinishExecute` true))
    (:`else`)))