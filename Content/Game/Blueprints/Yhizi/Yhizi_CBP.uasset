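; Yhizi is an AI enemy character that chases the player on sight.
; AI perception sets CanSeePlayer, and Tick uses a resettable DoOnce to enter Attack and issue AIMoveTo once per sighting.
; SetState writes the state to the blackboard and sets walk speed and CanCatch for Idle, Hunt or Attack.
; Catching is unfinished: CatchPlayer and the CatchBox overlap are empty, and the catch check and forced look-at logic are disconnected.
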(event `CatchPlayer`
  ;[1 1 1] Catch Player
)

(event `self.ReceiveBeginPlay`
  ;[1 1 1] BeginPlay
  (`self.AddMovementInput` (0.0 0.0 0.0)))

(event `self.ReceiveTick`
  (params (DeltaSeconds :type "Float (single-precision)"))
  ;[1 1 1] See Player
  (if (`self.CanSeePlayer?`)
    (`/Engine/EditorBlueprintResources/StandardMacros.DoOnce` false :!label _label
      (:`Completed`
        (`self.Set State` "NewEnumerator2")
        (`|AIMoveTo` self (0.0 0.0 0.0) (`GameplayStatics.GetPlayerCharacter` 0))))
    (else
      (goto _label :!via `Reset`))))

(event `self.AIPerception.OnTargetPerceptionUpdated`
  (params (Actor :type "Actor Object Reference") (Stimulus :type "AIStimulus Structure"))
  ;[1 1 1] See Player
  (`|ExecutionSequence`
    (:`then_1`
      (cast `/Game/Game/Blueprints/Player/Player_BP` Actor)
      (set `self.CanSeePlayer?` (`.bSuccessfullySensed` (break `AIStimulus` Stimulus))))))

(event `self.CatchBox.OnComponentBeginOverlap`
  (params (OverlappedComponent :type "PrimitiveComponent Object Reference") (OtherActor :type "Actor Object Reference") (OtherComp :type "PrimitiveComponent Object Reference") (OtherBodyIndex :type Integer) (bFromSweep :type Boolean) (SweepResult :type "HitResult Structure (by ref)")))

(fn `Set State`
  (params (`New State` :type "/Game/Game/Sosed/Enums/Yhizi_State Enum" :default "NewEnumerator0"))
  (bind _charactermovement (`self.CharacterMovement`))
  (`BlackboardComponent.SetValueAsEnum` (`AIBlueprintHelperLibrary.GetBlackboard` null) "State" `New State`)
  (switch `/Game/Game/Sosed/Enums/Yhizi_State` `New State`
    (:`NewEnumerator0`
      (set `CharacterMovementComponent.MaxWalkSpeed` 150.0 _charactermovement)
      (set `self.CanCatch?` false :!label _label))
    (:`NewEnumerator1`
      (set `CharacterMovementComponent.MaxWalkSpeed` 500.0 _charactermovement)
      (goto _label))
    (:`NewEnumerator2`
      (set `CharacterMovementComponent.MaxWalkSpeed` 550.0 _charactermovement)
      (set `self.CanCatch?` true))))

(fn `UserConstructionScript`)