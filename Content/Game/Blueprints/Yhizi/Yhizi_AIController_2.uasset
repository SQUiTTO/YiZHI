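; AI controller for the Yhizi_CBP_2 character, driving patrol and player detection through the Yhizi_BT_2 behavior tree.
; On BeginPlay it runs the tree and seeds the blackboard with the pawn's patrol path looping and wait time, plus a starting direction.
; Target perception updates for Player_BP set CanSeePlayer from any stimulus and print a debug string.
; An unconnected branch that separates noise investigation from sighting never runs.
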(event `self.ReceiveBeginPlay`
  (bind _returnvalue (`AIBlueprintHelperLibrary.GetBlackboard` null))
  (`self.RunBehaviorTree` "/Game/Game/Sosed/Behaviour/Yhizi_BT_2.Yhizi_BT_2")
  (bind _asyhizi_cbp_2 (cast `/Game/Game/Blueprints/Yhizi/Yhizi_CBP_2` (`self.K2_GetPawn`)))
  (bind _output_get (set `self.MyPawn` _asyhizi_cbp_2))
  (`BlackboardComponent.SetValueAsBool` (`AIBlueprintHelperLibrary.GetBlackboard` null) "PathLooping" (`/Game/Game/Sosed/Behaviour/PatrolPath.IsLooping` (`/Game/Game/Blueprints/Yhizi/Yhizi_CBP_2.PatrolPath` _output_get)))
  (`BlackboardComponent.SetValueAsInt` _returnvalue "Direction" 1)
  (`BlackboardComponent.SetValueAsFloat` _returnvalue "WaitTime" (`/Game/Game/Sosed/Behaviour/PatrolPath.WaitTime` (`/Game/Game/Blueprints/Yhizi/Yhizi_CBP_2.PatrolPath` (`self.MyPawn`)))))

(event `self.AIPerception.OnTargetPerceptionUpdated`
  (params (Actor :type "Actor Object Reference") (Stimulus :type "AIStimulus Structure"))
  (cast `/Game/Game/Blueprints/Player/Player_BP` Actor)
  (`BlackboardComponent.SetValueAsBool` (`AIBlueprintHelperLibrary.GetBlackboard` null) "CanSeePlayer" (`.bSuccessfullySensed` (break `AIStimulus` Stimulus)))
  (`KismetSystemLibrary.PrintString` "Hello"))

(event `self.AIPerception.OnPerceptionUpdated`
  (params (UpdatedActors :type "Array of Actor Object Reference (by ref)")))

(fn `UserConstructionScript`)