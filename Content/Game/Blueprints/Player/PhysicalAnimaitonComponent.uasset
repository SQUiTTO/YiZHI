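; Player actor component that sets up physical animation on the skeletal mesh of Player_BP.
; On BeginPlay it adds a PhysicalAnimationComponent to its owner at runtime, binds it to the player's mesh and caches both references.
; A placeholder-named CustomEvent turns off physics simulation for hand_r and the bodies below it.
; No animation profile or drive settings are applied here, and Tick is unused.
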(event `self.ReceiveBeginPlay`
  (bind _returnvalue (`|AddComponentByClass` (`self.GetOwner`) "/Script/Engine.PhysicalAnimationComponent"))
  (bind _output_get (set `self.Physical Animation Component` _returnvalue))
  (bind _asplayer_bp (cast `/Game/Game/Blueprints/Player/Player_BP` (`self.GetOwner`)))
  (bind _skeletalmesh (`/Game/Game/Blueprints/Player/Player_BP.SkeletalMesh` _asplayer_bp))
  (`PhysicalAnimationComponent.SetSkeletalMeshComponent` _output_get _skeletalmesh)
  (set `self.Skeletal Mesh` _skeletalmesh))

(event `CustomEvent`
  (`SkeletalMeshComponent.SetAllBodiesBelowSimulatePhysics` (`self.Skeletal Mesh`) "hand_r" false true))