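; Player character with Enhanced Input movement, look and jump, walk/idle camera shakes, and physics-based grabbing of interactable objects.
; Each tick a camera trace finds physics-simulating InteractionInterface components, highlights them via custom depth and shows their message on the HUD.
; The drag input asks the target to interact, then a PhysicsHandle grabs it at the hit point and follows the GRBhandle component until release.
; CalcCameraLean computes a yaw-based lean but is not called here.
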(event `self.ReceiveBeginPlay`
  (bind _returnvalue (`|CreateWidget` "/Game/Game/Widgets/HeadsUpDisplay.HeadsUpDisplay_C"))
  (bind _output_get (set `self.Heads Up Display` _returnvalue))
  (`UserWidget.AddToViewport` _output_get 0)
  (set `PlayerController.bEnableClickEvents` true (`GameplayStatics.GetPlayerController` 0)))

(event `self.ReceivePossessed`
  (params (NewController :type "Controller Object Reference"))
  (bind _asplayer_controller (cast `PlayerController` NewController))
  (`EnhancedInputSubsystemInterface.AddMappingContext` (pcsubsystem `EnhancedInputLocalPlayerSubsystem` _asplayer_controller) "/Game/Game/Inputs/InputMap_Player.InputMap_Player" 0 (struct))
  (`self.IdleShake`))

(event `EnhancedInput|/Game/Game/Inputs/IA_MoveForwardCC`
  (params (ActionValue :type "Float (double-precision)") (ElapsedSeconds :type "Float (double-precision)") (TriggeredSeconds :type "Float (double-precision)") (InputAction :type "InputAction Object Reference" :default "/Game/Game/Inputs/IA_MoveForwardCC.IA_MoveForwardCC"))
  (:`Triggered`
    (set `self.IsWalking` true)
    (`self.AddMovementInput` (`KismetMathLibrary.GetForwardVector` (`KismetMathLibrary.MakeRotator` 0.0 0.0 (.yaw (`self.GetControlRotation`)))) ActionValue)
    (if (and (not (`NavMovementComponent.IsFalling` (`self.CharacterMovement`))) (`self.IsWalking`)) :!label _label
      (`/Engine/EditorBlueprintResources/StandardMacros.DoOnce` false :!label _label_2
        (:`Completed`
          (`self.Start Camera Shake`)
          (goto _label_3 :!via `Reset`)))
      (else
        (`/Engine/EditorBlueprintResources/StandardMacros.DoOnce` false :!label _label_3
          (:`Completed`
            (`self.Stop Camera Shake`)
            (`self.IdleShake`)
            (goto _label_2 :!via `Reset`))))))
  (:`Completed`
    (set `self.IsWalking` false)
    (`KismetSystemLibrary.Delay` 0.1)
    (goto _label)))

(event `EnhancedInput|/Game/Game/Inputs/IA_MoveRightCC`
  (params (ActionValue :type "Float (double-precision)") (ElapsedSeconds :type "Float (double-precision)") (TriggeredSeconds :type "Float (double-precision)") (InputAction :type "InputAction Object Reference" :default "/Game/Game/Inputs/IA_MoveRightCC.IA_MoveRightCC"))
  (:`Triggered`
    (set `self.IsWalking` true)
    (`self.AddMovementInput` (`KismetMathLibrary.GetRightVector` (`KismetMathLibrary.MakeRotator` 0.0 0.0 (.yaw (`self.GetControlRotation`)))) ActionValue)
    (goto _label))
  (:`Completed`
    (set `self.IsWalking` false)
    (`KismetSystemLibrary.Delay` 0.1)
    (goto _label)))

(event `EnhancedInput|/Game/Game/Inputs/IA_TurnCC`
  (params (ActionValue :type "Float (double-precision)") (ElapsedSeconds :type "Float (double-precision)") (TriggeredSeconds :type "Float (double-precision)") (InputAction :type "InputAction Object Reference" :default "/Game/Game/Inputs/IA_TurnCC.IA_TurnCC"))
  (:`Triggered`
    (`self.AddControllerYawInput` ActionValue)
    (set `self.Turn` ActionValue)
    (set `self.IsTurning` true))
  (:`Completed`
    (set `self.IsTurning` false)))

(event `EnhancedInput|/Game/Game/Inputs/IA_LookUpCC`
  (params (ActionValue :type "Float (double-precision)") (ElapsedSeconds :type "Float (double-precision)") (TriggeredSeconds :type "Float (double-precision)") (InputAction :type "InputAction Object Reference" :default "/Game/Game/Inputs/IA_LookUpCC.IA_LookUpCC"))
  (:`Triggered`
    (`self.AddControllerPitchInput` ActionValue)))

(event `EnhancedInput|/Game/Game/Inputs/IA_DoorDragCC`
  (params (ActionValue :type Boolean) (ElapsedSeconds :type "Float (double-precision)") (TriggeredSeconds :type "Float (double-precision)") (InputAction :type "InputAction Object Reference" :default "/Game/Game/Inputs/IA_DoorDragCC.IA_DoorDragCC"))
  (:`Started`
    (bind _lookatcomponent (`self.LookAtComponent`)
      (:`then`
        (set `self.IsHolding` true)
        (bind _cangrab (message `/Game/Game/UI/InteractionInterface.InteractWith` (`ActorComponent.GetOwner` _lookatcomponent) self _lookatcomponent))
        (if _cangrab
          (if (`self.IsHoldingObject`)
            (`PhysicsHandleComponent.ReleaseComponent` (`self.PhysicsHandle`))
            (else
              (`self.Grab` 350.0)))
          (else
            (`PhysicsHandleComponent.ReleaseComponent` (`self.PhysicsHandle`)))))
      (:`else`)))
  (:`Completed`
    (if (`self.IsHoldingObject`)
      (set `self.IsHolding` false)
      (`PhysicsHandleComponent.ReleaseComponent` (`self.PhysicsHandle`)))))

(event `EnhancedInput|/Game/Game/Inputs/IA_JumpCC`
  (params (ActionValue :type Boolean) (ElapsedSeconds :type "Float (double-precision)") (TriggeredSeconds :type "Float (double-precision)") (InputAction :type "InputAction Object Reference" :default "/Game/Game/Inputs/IA_JumpCC.IA_JumpCC"))
  (:`Triggered`
    (`self.Jump`)))

(event `Start Camera Shake`
  ;[1 1 1] Camera Shake
  (bind _returnvalue (`PlayerCameraManager.StartCameraShake` :`self` (`GameplayStatics.GetPlayerCameraManager` 0) :`ShakeClass` "/Game/Game/Blueprints/CameraShake/CameraShake_Walk.CameraShake_Walk_C")))

(event `self.ReceiveTick`
  (params (DeltaSeconds :type "Float (single-precision)"))
  (bind (_returnvalue_location _returnvalue_rotation) (`KismetMathLibrary.BreakTransform` (`SceneComponent.K2_GetComponentToWorld` (`self.GRBhandle`))))
  (`self.InteractTrace` 350.0)
  (if (`self.IsHoldingObject`)
    (`PhysicsHandleComponent.SetTargetLocationAndRotation` (`self.PhysicsHandle`) _returnvalue_location _returnvalue_rotation)))

(event `Stop Camera Shake`
  ;[1 1 1] Camera Shake
  (`PlayerCameraManager.StopCameraShake` (`GameplayStatics.GetPlayerCameraManager` 0) (stale `Start Camera Shake` _returnvalue) false))

(event `IdleShake`
  ;[1 1 1] Camera Shake
  (`PlayerCameraManager.StartCameraShake` :`self` (`GameplayStatics.GetPlayerCameraManager` 0) :`ShakeClass` "/Game/Game/Blueprints/CameraShake/CameraShake_Idle.CameraShake_Idle_C")
  (`self.Stop Camera Shake`))

(fn `CalcCameraLean`
  (bind _returnvalue (`self.K2_GetActorRotation`))
  (bind (_returnvalue_roll _returnvalue_pitch _returnvalue_yaw) (`KismetMathLibrary.BreakRotator` (`KismetMathLibrary.NormalizedDeltaRotator` (`self.PreviousRotation`) _returnvalue)))
  (set `self.LeanAmount` (`KismetMathLibrary.FInterpTo` (`self.LeanAmount`) _returnvalue_yaw (`GameplayStatics.GetWorldDeltaSeconds`) 2.0))
  (bind _output_get (set `self.PreviousRotation` _returnvalue))
  (`KismetSystemLibrary.PrintString` (`KismetStringLibrary.Conv_RotatorToString` _output_get)))

(fn `Grab`
  (params (Range :type "Float (double-precision)"))
  (bind _returnvalue (`GameplayStatics.GetPlayerCameraManager` 0))
  (bind _returnvalue_2 (`self.K2_GetActorLocation` _returnvalue))
  (bind _outhit (`KismetSystemLibrary.LineTraceSingle` _returnvalue_2 (+ _returnvalue_2 (* (`self.GetActorForwardVector` _returnvalue) (`local.Range`))) "TraceTypeQuery1"))
  (bind (_bblockinghit _binitialoverlap _time _distance _location _impactpoint _normal) (`GameplayStatics.BreakHitResult` _outhit))
  (bind _returnvalue_3 (`KismetMathLibrary.MakeRotFromX` _normal))
  (`PhysicsHandleComponent.GrabComponentAtLocationWithRotation` (`self.PhysicsHandle`) (`self.LookAtComponent`) "None" _location _returnvalue_3)
  (`SceneComponent.K2_SetWorldLocationAndRotation` (`self.GRBhandle`) _location _returnvalue_3 false false))

(fn `InteractTrace`
  (params (Range :type "Float (double-precision)"))
  (locals (LocalHitResult :type "HitResult Structure") (NewLocalVar :type "Array of EObjectTypeQuery Enum"))
  (bind _returnvalue (`GameplayStatics.GetPlayerCameraManager` 0))
  (bind _returnvalue_2 (`self.K2_GetActorLocation` _returnvalue))
  (bind (_bblockinghit _binitialoverlap _time _distance _location _impactpoint _normal _impactnormal _physmat _hitactor _hitcomponent) (`GameplayStatics.BreakHitResult` (`local.LocalHitResult`)))
  (bind (_outhit _returnvalue_3) (`KismetSystemLibrary.LineTraceSingle` _returnvalue_2 (+ _returnvalue_2 (* (`self.GetActorForwardVector` _returnvalue) (`local.Range`))) "TraceTypeQuery1"))
  (if _returnvalue_3
    (set `local.LocalHitResult` _outhit)
    (bind (_bblockinghit_2 _binitialoverlap_2 _time_2 _distance_2 _location_2 _impactpoint_2 _normal_2 _impactnormal_2 _physmat_2 _hitactor_2 _hitcomponent_2) (`GameplayStatics.BreakHitResult` _outhit))
    (if (!= (`self.LookAtComponent`) _hitcomponent_2)
      (bind _lookatcomponent (`self.LookAtComponent`)
        (:`then`
          (`PrimitiveComponent.SetRenderCustomDepth` _lookatcomponent true))
        (:`else`
          _))
      (if (and (`KismetSystemLibrary.DoesImplementInterface` _hitactor_2 "/Game/Game/UI/InteractionInterface.InteractionInterface_C") (`SceneComponent.IsSimulatingPhysics` _hitcomponent_2 "None"))
        (bind (_lookatactor _lookatcomponent_2 _message) (message `/Game/Game/UI/InteractionInterface.LookAt` _hitactor self (`GameplayStatics.GetPlayerController` 0) _hitcomponent))
        (bind _output_get (set `self.LookAtComponent` _lookatcomponent_2))
        (`PrimitiveComponent.SetRenderCustomDepth` _output_get true)
        (`/Game/Game/Widgets/HeadsUpDisplay.DisplayMessage` (`self.Heads Up Display`) _message)
        (else
          (bind _lookatcomponent_3 (`self.LookAtComponent`)
            (:`then`
              (`PrimitiveComponent.SetRenderCustomDepth` _lookatcomponent_3 false)
              (set `self.LookAtComponent` null)
              (`/Game/Game/Widgets/HeadsUpDisplay.DisplayMessage` (`self.Heads Up Display`) ""))
            (:`else`)))))
    (else
      (bind _lookatcomponent_4 (`self.LookAtComponent`)
        (:`then`
          (`PrimitiveComponent.SetRenderCustomDepth` _lookatcomponent_4 false)
          (set `self.LookAtComponent` null)
          (`/Game/Game/Widgets/HeadsUpDisplay.DisplayMessage` (`self.Heads Up Display`) ""))
        (:`else`)))))

(fn `IsHoldingObject`
  (returns (ReturnValue :type Boolean))
  (return (`KismetSystemLibrary.IsValid` (`PhysicsHandleComponent.GetGrabbedComponent` (`self.PhysicsHandle`)))))

(fn `UserConstructionScript`)