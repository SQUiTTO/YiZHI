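; Physics-driven door that the player can grab, showing a "Grab Door" prompt when looked at.
; Interacting lowers the mesh's mass and angular damping so it can swing.
; Overlap while the player is holding restores the heavy mass and stops the reset timeline.
; After overlap ends, a short delay restores mass and high damping, then plays the timeline that lerps the door's relative rotation back to zero.
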(event `self.ReceiveBeginPlay`
  (bind _asplayer_bp (cast `/Game/Game/Blueprints/Player/Player_BP` (`GameplayStatics.GetPlayerCharacter` 0)))
  (set `self.As Player BP` _asplayer_bp))

(event `self.ReceiveTick`
  (params (DeltaSeconds :type "Float (single-precision)")))

(event `self.ReceiveActorBeginOverlap`
  (params (OtherActor :type "Actor Object Reference"))
  (bind _sm_door (`self.SM_Door`))
  (if (`/Game/Game/Blueprints/Player/Player_BP.IsHolding` (`self.As Player BP`))
    (`KismetSystemLibrary.PrintString` "HOLDING")
    (`PrimitiveComponent.SetMassOverrideInKg` (`self.SM_Door`) "None" 1000.0 true)
    (bind (_direction _reset) (`Timeline|Timeline` :!via `Stop` :!label _label)
      (:`Update`
        (`SceneComponent.K2_SetRelativeRotation` _sm_door (`KismetMathLibrary.RLerp` (`SceneComponent.RelativeRotation` _sm_door) (struct) _reset true) false false)))))

(event `EnhancedInput|/Game/Game/Inputs/IA_DoorDragCC`
  (params (ActionValue :type Boolean) (ElapsedSeconds :type "Float (double-precision)") (TriggeredSeconds :type "Float (double-precision)") (InputAction :type "InputAction Object Reference" :default "/Game/Game/Inputs/IA_DoorDragCC.IA_DoorDragCC")))

(event `self.ReceiveActorEndOverlap`
  (params (OtherActor :type "Actor Object Reference"))
  (bind _sm_door (`self.SM_Door`))
  (`KismetSystemLibrary.Delay` 3.0)
  (`KismetSystemLibrary.PrintString` "NOTHOLDING")
  (`PrimitiveComponent.SetMassOverrideInKg` _sm_door "None" 1000.0 true)
  (`PrimitiveComponent.SetAngularDamping` _sm_door 1000.0)
  (goto _label :!via `PlayFromStart`))

(fn `InteractWith`
  (params (Interactor :type "/Game/Game/Blueprints/Player/Player_BP Object Reference") (HitComponent :type "PrimitiveComponent Object Reference"))
  (returns (CanGrab :type Boolean))
  (bind _sm_door (`self.SM_Door`))
  (`PrimitiveComponent.SetMassOverrideInKg` _sm_door "None" 20.0 true)
  (`PrimitiveComponent.SetAngularDamping` _sm_door 10.0)
  (return true))

(fn `LookAt`
  (params (Interactor :type "/Game/Game/Blueprints/Player/Player_BP Object Reference") (PlayerController :type "PlayerController Object Reference") (HitComponent :type "PrimitiveComponent Object Reference"))
  (returns (LookAtActor :type "Actor Object Reference") (LookAtComponent :type "PrimitiveComponent Object Reference") (Message :type Text))
  (return self HitComponent "Grab Door"))

(fn `UserConstructionScript`)