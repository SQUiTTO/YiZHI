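; Hinged door that the player drags open and shut by holding the drag input and turning, using direct yaw rotation instead of physics.
; A short camera line trace on press confirms the target door, then the player's turn value drives the clamped mesh yaw.
; Facing relative to the door sets the turn sign once per drag, and a Flipped option mirrors the swing.
; Leaving the door's overlap volume can trigger a delayed Timeline that eases it back to zero rotation.
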(event `self.ReceiveBeginPlay`
  ;[1 1 1] Get Player Input
  (`self.EnableInput` (`GameplayStatics.GetPlayerController` 0))
  (if (`self.Flipped`)
    (set `self.Default Sensitivity` (* (`self.Default Sensitivity`) -1.0))
    (set `self.OpenAngle` 0.0)
    (set `self.ClosedAngle` -90.0)))

(event `EnhancedInput|/Game/Game/Inputs/IA_DoorDragCC`
  (params (ActionValue :type Boolean) (ElapsedSeconds :type "Float (double-precision)") (TriggeredSeconds :type "Float (double-precision)") (InputAction :type "InputAction Object Reference" :default "/Game/Game/Inputs/IA_DoorDragCC.IA_DoorDragCC"))
  ;[1 1 1] Mouse Drag Door Opening
  (:`Triggered`
    (if (and (`self.IsLookingAtDoor?`) (`self.IsHoldingLMB?`) (`/Game/Game/Blueprints/Player/Player_BP.IsTurning` (`self.As Player BP`)) (== (`self.Hit Actor`) self))
      (`|ExecutionSequence`
        (:`then_0`
          (`/Engine/EditorBlueprintResources/StandardMacros.DoOnce` false :!label _label
            (:`Completed`
              (`self.LookRotation`))))
        (:`then_1`
          (`self.UpdateSlide`)))))
  (:`Started`
    (set `self.IsHoldingLMB?` true)
    (bind _asplayer_bp (cast `/Game/Game/Blueprints/Player/Player_BP` (`GameplayStatics.GetPlayerCharacter` 0)))
    (set `self.As Player BP` _asplayer_bp)
    (bind _fp_camera (`/Game/Game/Blueprints/Player/Player_BP.FP_Camera` _asplayer_bp))
    (bind _returnvalue (`SceneComponent.K2_GetComponentLocation` _fp_camera))
    (bind (_outhit _returnvalue_2) (`KismetSystemLibrary.LineTraceSingleForObjects` _returnvalue (+ _returnvalue (* (`SceneComponent.GetForwardVector` _fp_camera) 175.0)) (`|MakeArray` "ObjectTypeQuery2" :!type "EObjectTypeQuery Enum") false (`|MakeArray` (`self.As Player BP`) :!type "Actor Object Reference") "ForDuration" false))
    (if _returnvalue_2
      (bind (_bblockinghit _binitialoverlap _time _distance _location _impactpoint _normal _impactnormal _physmat _hitactor) (`GameplayStatics.BreakHitResult` _outhit))
      (set `self.Hit Actor` _hitactor)
      (if (== self _hitactor)
        (cast `/Game/Game/Blueprints/Environment/Door/NewDoor_NotPhysics_BP` _hitactor)
        (set `self.IsLookingAtDoor?` true))
      (else
        (set `self.IsLookingAtDoor?` false))))
  (:`Completed`
    (`|ExecutionSequence`
      (:`then_0`
        (goto _label :!via `Reset`))
      (:`then_1`
        (set `self.IsHoldingLMB?` false)
        (`self.UpdateSlide`)))))

(event `self.InDoorSpace.OnComponentEndOverlap`
  (params (OverlappedComponent :type "PrimitiveComponent Object Reference") (OtherActor :type "Actor Object Reference") (OtherComp :type "PrimitiveComponent Object Reference") (OtherBodyIndex :type Integer))
  (bind _sm_door_01 (`self.SM_Door_01`))
  ;[1 1 1] Automatic Close Door Once Out of Range
  (if (== self (`self.Hit Actor`))
    (`KismetSystemLibrary.Delay` 4.0)
    (if (and (not (`self.IsHoldingLMB?`)) (`self.IsLookingAtDoor?`))
      (bind (_direction _reset) (`Timeline|Timeline` :!via `PlayFromStart`)
        (:`Update`
          (`SceneComponent.K2_SetRelativeRotation` _sm_door_01 (`KismetMathLibrary.RLerp` (`SceneComponent.RelativeRotation` _sm_door_01) (struct) _reset true) false false))))))

(fn `LookRotation`
  (bind _default_sensitivity (`self.Default Sensitivity`))
  (bind _returnvalue (`self.GetActorForwardVector` (`self.As Player BP`)))
  (if (< (`KismetMathLibrary.Dot_VectorVector` (`KismetMathLibrary.Normal` (- (`SceneComponent.GetForwardVector` (`self.DefaultSceneRoot`)) _returnvalue)) _returnvalue) -0.5)
    (set `self.TurnSensitivity` (* _default_sensitivity -1.0))
    (else
      (set `self.TurnSensitivity` _default_sensitivity))))

(fn `UpdateSlide`
  (locals (DragDoorRot :type "Rotator Structure" :default (struct)))
  (bind (_relativerotation_roll _relativerotation_pitch _relativerotation_yaw) (`KismetMathLibrary.BreakRotator` (`SceneComponent.RelativeRotation` (`self.SM_Door_01`))))
  (if true
    (`SceneComponent.K2_SetRelativeRotation` (`self.SM_Door_01`) (`KismetMathLibrary.MakeRotator` 0.0 0.0 (`KismetMathLibrary.FClamp` (+ (* (`/Game/Game/Blueprints/Player/Player_BP.Turn` (`self.As Player BP`)) (`self.TurnSensitivity`)) _relativerotation_yaw) (`self.ClosedAngle`) (`self.OpenAngle`))) false false)
    (if (`self.IsHoldingLMB?`)
      _)))

(fn `UserConstructionScript`)