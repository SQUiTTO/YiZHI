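; Item_BP is an interactable item actor that destroys itself when the player interacts with it in range.
; It caches the Player_BP reference at BeginPlay, then uses sphere overlaps to show or hide a widget and print debug messages.
; Tick is enabled only while the player overlaps, polling IsInteracting and firing a one-shot, briefly delayed destroy.
; The item itself grants nothing to the player.
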(event `self.ReceiveBeginPlay`
  (`self.Reference Setup`)
  (`self.SetActorTickEnabled` false)
  (`SceneComponent.SetVisibility` (`self.Widget`) false false))

(event `self.Sphere1.OnComponentBeginOverlap`
  (params (OverlappedComponent :type "PrimitiveComponent Object Reference") (OtherActor :type "Actor Object Reference") (OtherComp :type "PrimitiveComponent Object Reference") (OtherBodyIndex :type Integer) (bFromSweep :type Boolean) (SweepResult :type "HitResult Structure (by ref)"))
  (if (== OtherActor (`self.Player`))
    (`KismetSystemLibrary.PrintString` "You are in my DOMAIN!")
    (`SceneComponent.SetVisibility` (`self.Widget`) true false)
    (`self.SetActorTickEnabled` true)))

(event `self.Sphere1.OnComponentEndOverlap`
  (params (OverlappedComponent :type "PrimitiveComponent Object Reference") (OtherActor :type "Actor Object Reference") (OtherComp :type "PrimitiveComponent Object Reference") (OtherBodyIndex :type Integer))
  (if (== OtherActor (`self.Player`))
    (`KismetSystemLibrary.PrintString` "Get the FUCK OUT!")
    (`SceneComponent.SetVisibility` (`self.Widget`) false false)
    (`self.SetActorTickEnabled` false)))

(event `self.ReceiveTick`
  (params (DeltaSeconds :type "Float (single-precision)"))
  (if (`/Game/Game/Blueprints/Player/Player_BP.IsInteracting` (`self.Player`))
    (`/Engine/EditorBlueprintResources/StandardMacros.DoOnce` false
      (:`Completed`
        (`KismetSystemLibrary.Delay` 0.1)
        (`self.K2_DestroyActor`)))))

(fn `Reference Setup`
  (bind _asplayer_bp (cast `/Game/Game/Blueprints/Player/Player_BP` (`GameplayStatics.GetPlayerCharacter` 0)))
  (set `self.Player` _asplayer_bp))

(fn `UserConstructionScript`)