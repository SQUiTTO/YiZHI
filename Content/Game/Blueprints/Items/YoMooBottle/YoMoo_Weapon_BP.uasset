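; YoMoo bottle weapon that the player picks up, carries in the right hand and throws to create a splash.
; Sphere overlap shows a prompt widget and enables Tick, which watches for interaction to attach the bottle and enable input.
; Throwing detaches it and applies a camera-forward physics impulse.
; Tick then polls the capsule for static world meshes, spawning YooMoo_Splash_BP and destroying the bottle on contact.
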(event `self.ReceiveBeginPlay`
  ;[1 1 1] Initialze Blueprint
  (`self.CommunicationSetup`)
  (`SceneComponent.SetVisibility` (`self.Widget`) false false)
  (`self.SetActorTickEnabled` false)
  (`PrimitiveComponent.SetSimulatePhysics` (`self.Bottle`) false)
  (`PrimitiveComponent.SetCollisionEnabled` (`self.Capsule`) "NoCollision"))

(event `self.Sphere.OnComponentBeginOverlap`
  (params (OverlappedComponent :type "PrimitiveComponent Object Reference") (OtherActor :type "Actor Object Reference") (OtherComp :type "PrimitiveComponent Object Reference") (OtherBodyIndex :type Integer) (bFromSweep :type Boolean) (SweepResult :type "HitResult Structure (by ref)"))
  ;[1 1 1] Overlapping OnGround
  (if (== OtherActor (`self.Player`))
    (`SceneComponent.SetVisibility` (`self.Widget`) true false)
    (`self.SetActorTickEnabled` true)))

(event `self.Sphere.OnComponentEndOverlap`
  (params (OverlappedComponent :type "PrimitiveComponent Object Reference") (OtherActor :type "Actor Object Reference") (OtherComp :type "PrimitiveComponent Object Reference") (OtherBodyIndex :type Integer))
  ;[1 1 1] End Overlapping On Ground
  (if (== OtherActor (`self.Player`))
    (`SceneComponent.SetVisibility` (`self.Widget`) false false)
    (`self.SetActorTickEnabled` false)))

(event `EnhancedInput|/Game/Game/Inputs/IA_ThrowWeaponCC`
  (params (ActionValue :type Boolean) (ElapsedSeconds :type "Float (double-precision)") (TriggeredSeconds :type "Float (double-precision)") (InputAction :type "InputAction Object Reference" :default "/Game/Game/Inputs/IA_ThrowWeaponCC.IA_ThrowWeaponCC"))
  (bind _bottle (`self.Bottle`))
  ;[1 1 1] Throwing the Bottle
  (:`Started`
    (`/Engine/EditorBlueprintResources/StandardMacros.IsValid` self
      (:`Is Valid`
        (set `/Game/Game/Blueprints/Player/Player_BP.HasBottleWeapon` false (`self.Player`))
        (set `self.ThrownBottle` true)
        (`self.K2_DetachFromActor` self "KeepWorld" "KeepWorld" "KeepWorld")
        (`PrimitiveComponent.SetCollisionEnabled` (`self.Sphere`) "NoCollision")
        (`PrimitiveComponent.SetSimulatePhysics` _bottle true)
        (`PrimitiveComponent.AddImpulse` _bottle (* (`SceneComponent.GetForwardVector` (`/Game/Game/Blueprints/Player/Player_BP.FP_Camera` (`self.Player`))) 2000.0) "None" false)
        (`PrimitiveComponent.SetCollisionEnabled` (`self.Capsule`) "QueryOnly")
        (`self.SetActorTickEnabled` true)))))

(event `self.ReceiveTick`
  (params (DeltaSeconds :type "Float (single-precision)"))
  (bind _player (`self.Player`))
  (bind _capsule (`self.Capsule`))
  ;[1 1 1] Event Tick
  (if (and (`/Game/Game/Blueprints/Player/Player_BP.IsInteracting` _player) (not (`/Game/Game/Blueprints/Player/Player_BP.HasBottleWeapon` _player)))
    (`/Engine/EditorBlueprintResources/StandardMacros.DoOnce` false
      (:`Completed`
        (`KismetSystemLibrary.Delay` 0.2)
        (set `/Game/Game/Blueprints/Player/Player_BP.HasBottleWeapon` true (`self.Player`))
        (`SceneComponent.SetVisibility` (`self.Widget`) false false)
        (`self.K2_AttachToComponent` (`/Game/Game/Blueprints/Player/Player_BP.SkeletalMesh` (`self.Player`)) "handweapon_r" "SnapToTarget" "SnapToTarget" "SnapToTarget")
        (`self.EnableInput` (`GameplayStatics.GetPlayerController` 0))))
    (elif (`self.ThrownBottle`)
      (bind (_outactors _returnvalue) (`KismetSystemLibrary.ComponentOverlapActors` _capsule (`SceneComponent.K2_GetComponentToWorld` _capsule) (`|MakeArray` "ObjectTypeQuery1" :!type "EObjectTypeQuery Enum") "/Script/Engine.StaticMeshActor"))
      (if _returnvalue
        (`/Engine/EditorBlueprintResources/StandardMacros.DoOnce` false
          (:`Completed`
            (`self.SetActorTickEnabled` false)
            (set `self.ThrownBottle` false)
            (`KismetSystemLibrary.Delay` 0.05)
            (`|SpawnActorFromClass` "/Game/Game/Blueprints/Items/YoMooBottle/YooMoo_Splash_BP.YooMoo_Splash_BP_C" (`SceneComponent.K2_GetComponentToWorld` (`self.Capsule`)) "Undefined" "OverrideRootScale" null null)
            (`self.K2_DestroyActor`)))))))

(fn `CommunicationSetup`
  (bind _asplayer_bp (cast `/Game/Game/Blueprints/Player/Player_BP` (`GameplayStatics.GetPlayerCharacter` 0)))
  (set `self.Player` _asplayer_bp))

(fn `UserConstructionScript`)