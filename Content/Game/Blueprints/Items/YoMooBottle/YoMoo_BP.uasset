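; YoMoo_BP is a bottle pickup that grants the player the bottle weapon.
; Overlapping its sphere shows a prompt widget and enables Tick, so interaction is only polled while the player is in range.
; When the player interacts without already holding a bottle, a DoOnce-guarded short delay sets HasBottleWeapon, destroys the pickup and spawns YoMoo_Weapon_BP at the world origin.
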(event `self.ReceiveBeginPlay`
  (`self.ReferenceSetup`)
  (`SceneComponent.SetVisibility` (`self.Widget`) false false)
  (`self.SetActorTickEnabled` false))

(event `self.Sphere.OnComponentBeginOverlap`
  (params (OverlappedComponent :type "PrimitiveComponent Object Reference") (OtherActor :type "Actor Object Reference") (OtherComp :type "PrimitiveComponent Object Reference") (OtherBodyIndex :type Integer) (bFromSweep :type Boolean) (SweepResult :type "HitResult Structure (by ref)"))
  (if (== OtherActor (`self.Player`))
    (`SceneComponent.SetVisibility` (`self.Widget`) true false)
    (`self.SetActorTickEnabled` true)))

(event `self.Sphere.OnComponentEndOverlap`
  (params (OverlappedComponent :type "PrimitiveComponent Object Reference") (OtherActor :type "Actor Object Reference") (OtherComp :type "PrimitiveComponent Object Reference") (OtherBodyIndex :type Integer))
  (if (== OtherActor (`self.Player`))
    (`SceneComponent.SetVisibility` (`self.Widget`) false false)
    (`self.SetActorTickEnabled` false)))

(event `self.ReceiveTick`
  (params (DeltaSeconds :type "Float (single-precision)"))
  (bind _player (`self.Player`))
  (if (and (`/Game/Game/Blueprints/Player/Player_BP.IsInteracting` _player) (not (`/Game/Game/Blueprints/Player/Player_BP.HasBottleWeapon` _player)))
    (`/Engine/EditorBlueprintResources/StandardMacros.DoOnce` false
      (:`Completed`
        (`KismetSystemLibrary.Delay` 0.2)
        (set `/Game/Game/Blueprints/Player/Player_BP.HasBottleWeapon` true (`self.Player`))
        (`SceneComponent.SetVisibility` (`self.Widget`) false false)
        (`self.SetActorTickEnabled` false)
        (`self.K2_DestroyActor`)
        (`|SpawnActorFromClass` "/Game/Game/Blueprints/Items/YoMooBottle/YoMoo_Weapon_BP.YoMoo_Weapon_BP_C" (`KismetMathLibrary.MakeTransform` (0.0 0.0 0.0)) "Undefined" "OverrideRootScale" null null)))))

(fn `ReferenceSetup`
  (bind _asplayer_bp (cast `/Game/Game/Blueprints/Player/Player_BP` (`GameplayStatics.GetPlayerCharacter` 0)))
  (set `self.Player` _asplayer_bp))

(fn `UserConstructionScript`)