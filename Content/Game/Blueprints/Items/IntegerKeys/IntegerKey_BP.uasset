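; IntegerKey_BP is a key pickup that adds one to the player's DoorKeys count.
; A sphere overlap with the player shows the widget and enables Tick, which polls the player's IsInteracting flag only while in range.
; On interact, a DoOnce guards the increment, then the key prints the new count and destroys itself after a short delay.
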(event `self.ReceiveBeginPlay`
  (`self.Reference Setup`)
  (`self.SetActorTickEnabled` false)
  (`SceneComponent.SetVisibility` (`self.Widget`) false false))

(event `self.Sphere.OnComponentBeginOverlap`
  (params (OverlappedComponent :type "PrimitiveComponent Object Reference") (OtherActor :type "Actor Object Reference") (OtherComp :type "PrimitiveComponent Object Reference") (OtherBodyIndex :type Integer) (bFromSweep :type Boolean) (SweepResult :type "HitResult Structure (by ref)"))
  (if (== OtherActor (`self.Player`))
    (`SceneComponent.SetVisibility` (`self.Widget`) true false)
    (`self.SetActorTickEnabled` true)))

(event `self.Sphere.OnComponentEndOverlap`
  (params (OverlappedComponent :type "PrimitiveComponent Object Reference") (OtherActor :type "Actor Object Reference") (OtherComp :type "PrimitiveComponent Object Reference") (OtherBodyIndex :type Integer))
  (if (== OtherActor (`self.Player`))
    (`SceneComponent.SetVisibility` (`self.Widget`) false false)
    (`self.SetActorTickEnabled` false)))

(event `self.ReceiveTick`
  (params (DeltaSeconds :type "Float (single-precision)"))
  (bind _player (`self.Player`))
  (if (`/Game/Game/Blueprints/Player/Player_BP.IsInteracting` (`self.Player`))
    (`/Engine/EditorBlueprintResources/StandardMacros.DoOnce` false
      (:`Completed`
        (bind _result (`/Engine/EditorBlueprintResources/StandardMacros.IncrementInt` (`/Game/Game/Blueprints/Player/Player_BP.DoorKeys` _player))
          (:`  `
            (bind _output_get (set `/Game/Game/Blueprints/Player/Player_BP.DoorKeys` _result _player))
            (`KismetSystemLibrary.PrintString` (`KismetStringLibrary.Conv_IntToString` _output_get))
            (`KismetSystemLibrary.Delay` 0.2)
            (`self.K2_DestroyActor`)
            (`self.SetActorTickEnabled` false)))))))

(fn `Reference Setup`
  (bind _asplayer_bp (cast `/Game/Game/Blueprints/Player/Player_BP` (`GameplayStatics.GetPlayerCharacter` 0)))
  (set `self.Player` _asplayer_bp))

(fn `UserConstructionScript`)